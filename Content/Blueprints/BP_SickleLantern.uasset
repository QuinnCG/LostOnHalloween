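; Sickle Lantern enemy character that plays a spawn montage before its parent Tick logic and melee attack become active.
; Tick starts an attack montage when the player is near, raising walk speed until a "Damage" notify slows it and damages the player if still close.
; On health component death, it disables collision, halts by issuing an AI move to its own location, and destroys itself after a delay.
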(event `self.ReceiveBeginPlay`
  (`|PlayMontage` (`self.Mesh`) "/Game/Animations/M_SickleLanternSpawn.M_SickleLanternSpawn"
    (:`OnCompleted`
      _)
    (:`OnBlendOut`
      _)
    (:`OnInterrupted`
      _))
  (`KismetSystemLibrary.Delay` 0.2)
  (set `self.IsSpawned` true))

(event `self.ReceiveTick`
  (params (DeltaSeconds :type "Float (single-precision)"))
  (bind _returnvalue (`self.GetController`))
  (if (`self.IsSpawned`)
    (`parent.ReceiveTick` DeltaSeconds)
    (if (and (< (`self.GetDistanceTo` (`GameplayStatics.GetPlayerPawn` 0)) 350.0) (not (`self.IsAttacking`)))
      (set `self.IsAttacking` true)
      (bind _notifyname (`|PlayMontage` (`self.Mesh`) "/Game/Animations/M_SickleLanternAttack.M_SickleLanternAttack")
        (:`then`
          (set `CharacterMovementComponent.MaxWalkSpeed` 400.0 (`self.CharacterMovement`)))
        (:`OnCompleted`
          (set `self.IsAttacking` false)
          (set `CharacterMovementComponent.MaxWalkSpeed` (`self.WalkSpeed`) (`self.CharacterMovement`)))
        (:`OnNotifyBegin`
          (if (== _notifyname "Damage")
            (set `CharacterMovementComponent.MaxWalkSpeed` 200.0 (`self.CharacterMovement`))
            (if (< (`self.GetDistanceTo` (`GameplayStatics.GetPlayerPawn` 0)) 150.0)
              (`GameplayStatics.ApplyDamage` (`GameplayStatics.GetPlayerPawn` 0) (`self.Damage`) _returnvalue _returnvalue))))))))

(event `self.BP_HealthComponent.OnDeath`
  (set `self.IsDead` true)
  (set `self.IsSpawned` false)
  (`PrimitiveComponent.SetCollisionEnabled` (`self.CapsuleComponent`) "NoCollision")
  (`|AIMoveTo` null (`self.K2_GetActorLocation`) null 5.0 true
    (:`then`
      (`KismetSystemLibrary.Delay` 10.0)
      (`self.K2_DestroyActor`))))

(fn `UserConstructionScript`
  (`parent.UserConstructionScript`)
  (set `CharacterMovementComponent.MaxWalkSpeed` (`self.WalkSpeed`) (`self.CharacterMovement`)))