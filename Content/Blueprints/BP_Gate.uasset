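; BP_Gate is a double gate that swings shut once when the player character enters its trigger.
; Overlap on CloseTrigger calls Close, which the IsClosed flag limits to a single run.
; The CloseAnim timeline's Angle track is remapped to separate yaw ranges to rotate the Right and Left leaves to their closed positions.
; The graph has no logic to reopen the gate.
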(event `Close`
  (if (not (`self.IsClosed`))
    (set `self.IsClosed` true)
    (bind (_direction _angle) (`Timeline|CloseAnim` :!via `PlayFromStart`)
      (:`Update`
        (`SceneComponent.K2_SetRelativeRotation` (`self.Right`) (`KismetMathLibrary.MakeRotator` 0.0 0.0 (`KismetMathLibrary.MapRangeClamped` _angle 0.0 1.0 -257.0 -180.0)) false false)
        (`SceneComponent.K2_SetRelativeRotation` (`self.Left`) (`KismetMathLibrary.MakeRotator` 0.0 0.0 (`KismetMathLibrary.MapRangeClamped` _angle 0.0 1.0 75.0)) false false)))))

(event `self.CloseTrigger.OnActorBeginOverlap`
  (params (OverlappedActor :type "Actor Object Reference") (OtherActor :type "Actor Object Reference"))
  (cast `/Game/Blueprints/BP_PlayerCharacter` OtherActor)
  (`self.Close`))

(fn `UserConstructionScript`)