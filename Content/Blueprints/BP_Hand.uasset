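; BP_Hand is a hand actor that turns on yaw to face the player and registers itself as grabbing when the player comes close.
; Overlap with DetectionSphere toggles CanDetect, which enables a per-Tick distance check against GrabDistance.
; Two alternating gates act as a latch, incrementing the player character's HandGrabCount once within range and decrementing it once beyond range while detection is active.
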(event `self.ReceiveTick`
  (params (DeltaSeconds :type "Float (single-precision)"))
  (bind _handgrabcount (`/Game/Blueprints/BP_PlayerCharacter.HandGrabCount` (cast `/Game/Blueprints/BP_PlayerCharacter` (`GameplayStatics.GetPlayerPawn` 0) :!pure true)))
  (bind (_returnvalue_roll _returnvalue_pitch _returnvalue_yaw) (`KismetMathLibrary.BreakRotator` (`KismetMathLibrary.MakeRotFromX` (- (`self.K2_GetActorLocation` (`GameplayStatics.GetPlayerPawn` 0)) (`self.K2_GetActorLocation`)))))
  (`|ExecutionSequence`
    (:`then_0`
      (`self.K2_SetActorRotation` (`KismetMathLibrary.MakeRotator` 0.0 0.0 _returnvalue_yaw)))
    (:`then_1`
      (if (`self.CanDetect`)
        (bind _output_get (set `self.Distance` (`KismetMathLibrary.Vector_Distance` (`self.K2_GetActorLocation` (`GameplayStatics.GetPlayerPawn` 0)) (`self.K2_GetActorLocation`))))
        (if (< _output_get (`self.GrabDistance`))
          (`/Engine/EditorBlueprintResources/StandardMacros.Gate` false :!label _label
            (:`Exit`
              (`|ExecutionSequence`
                (:`then_0`
                  (goto _label :!via `Close`))
                (:`then_1`
                  (`/Engine/EditorBlueprintResources/StandardMacros.IncrementInt` _handgrabcount))
                (:`then_2`
                  (goto _label_2 :!via `Open`)))))
          (else
            (`/Engine/EditorBlueprintResources/StandardMacros.Gate` true :!label _label_2
              (:`Exit`
                (`|ExecutionSequence`
                  (:`then_0`
                    (goto _label_2 :!via `Close`))
                  (:`then_1`
                    (`/Engine/EditorBlueprintResources/StandardMacros.DecrementInt` _handgrabcount))
                  (:`then_2`
                    (goto _label :!via `Open`)))))))
        (else
          (set `self.Distance` 1e+16))))))

(event `self.DetectionSphere.OnComponentBeginOverlap`
  (params (OverlappedComponent :type "PrimitiveComponent Object Reference") (OtherActor :type "Actor Object Reference") (OtherComp :type "PrimitiveComponent Object Reference") (OtherBodyIndex :type Integer) (bFromSweep :type Boolean) (SweepResult :type "HitResult Structure (by ref)"))
  (cast `/Game/Blueprints/BP_PlayerCharacter` OtherActor)
  (set `self.CanDetect` true))

(event `self.DetectionSphere.OnComponentEndOverlap`
  (params (OverlappedComponent :type "PrimitiveComponent Object Reference") (OtherActor :type "Actor Object Reference") (OtherComp :type "PrimitiveComponent Object Reference") (OtherBodyIndex :type Integer))
  (cast `/Game/Blueprints/BP_PlayerCharacter` OtherActor)
  (set `self.CanDetect` false))

(fn `UserConstructionScript`)