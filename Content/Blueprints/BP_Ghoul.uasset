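; BP_Ghoul is a melee enemy that spawns facing the player and self-destructs after 60 seconds.
; A spawn montage pins it in place until finished, with a notify enabling gravity and collision.
; Tick runs parent logic, starts in-range attack montages whose notify slows it and applies damage, and plays movement-based voice sounds.
; Health component events drive hurt sounds and death, which disables collision, locks yaw and delays destruction.
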(event `self.ReceiveBeginPlay`
  (bind (_returnvalue_roll _returnvalue_pitch _returnvalue_yaw) (`KismetMathLibrary.BreakRotator` (`KismetMathLibrary.MakeRotFromX` (`KismetMathLibrary.Normal` (- (`self.K2_GetActorLocation` (`GameplayStatics.GetPlayerPawn` 0)) (`self.K2_GetActorLocation`))))))
  (`|ExecutionSequence`
    (:`then_0`
      (set `self.Pos` (`self.K2_GetActorLocation`))
      (`SceneComponent.K2_SetWorldRotation` (`self.CapsuleComponent`) (`KismetMathLibrary.MakeRotator` 0.0 0.0 _returnvalue_yaw) false false))
    (:`then_1`
      (bind _notifyname (`|PlayMontage` (`self.Mesh`) "/Game/Animations/GhoulSpawn_Montage.GhoulSpawn_Montage")
        (:`OnCompleted`
          (set `self.IsSpawning` false :!label _label))
        (:`OnBlendOut`
          (goto _label))
        (:`OnInterrupted`
          (goto _label))
        (:`OnNotifyBegin`
          (if (== _notifyname "Collide")
            (`PrimitiveComponent.SetEnableGravity` (`self.CapsuleComponent`) true)
            (`PrimitiveComponent.SetCollisionEnabled` (`self.CapsuleComponent`) "QueryAndPhysics")))))
    (:`then_2`
      (`KismetSystemLibrary.Delay` 60.0)
      (`self.K2_DestroyActor`))))

(event `self.ReceiveTick`
  (params (DeltaSeconds :type "Float (single-precision)"))
  (bind _returnvalue (`self.GetController`))
  (bind _charactermovement (`self.CharacterMovement`))
  (bind _returnvalue_2 (`SceneComponent.K2_GetComponentLocation` (`self.Mouth`)))
  (if (`self.IsDead`)
    (`self.K2_SetActorRotation` (`KismetMathLibrary.MakeRotator` 0.0 0.0 (`self.DeathYaw`)))
    (else
      (`|ExecutionSequence`
        (:`then_0`
          (if (`self.IsSpawning`)
            (`SceneComponent.K2_SetWorldLocation` (`self.CapsuleComponent`) (`self.Pos`) false true)
            (else
              (`parent.ReceiveTick` DeltaSeconds)
              (if (< (`self.GetDistanceTo` (`GameplayStatics.GetPlayerPawn` 0)) (`self.AttackRange`))
                (if (not (and (`self.IsAttacking`) (`self.IsSpawning`)))
                  (set `self.IsAttacking` true)
                  (bind _notifyname (`|PlayMontage` (`self.Mesh`) "/Game/Animations/GhoulAttack_Montage.GhoulAttack_Montage" 0.8)
                    (:`OnCompleted`
                      (`KismetSystemLibrary.Delay` (`self.AttackCooldown`) :!label _label_2)
                      (set `self.IsAttacking` false)
                      (set `CharacterMovementComponent.MaxWalkSpeed` 300.0 _charactermovement))
                    (:`OnBlendOut`
                      (goto _label_2))
                    (:`OnInterrupted`
                      (goto _label_2))
                    (:`OnNotifyBegin`
                      (if (== _notifyname "Damage")
                        (`|ExecutionSequence`
                          (:`then_0`
                            (set `CharacterMovementComponent.MaxWalkSpeed` 125.0 _charactermovement))
                          (:`then_1`
                            (if (< (`self.GetDistanceTo` (`GameplayStatics.GetPlayerPawn` 0)) (`self.DamageRange`))
                              (`GameplayStatics.ApplyDamage` (`GameplayStatics.GetPlayerPawn` 0) (`self.Damage`) _returnvalue _returnvalue)))
                          (:`then_2`
                            (`GameplayStatics.PlaySoundAtLocation` "/Game/Audio/Cues/C_GhoulAttack.C_GhoulAttack" (`SceneComponent.K2_GetComponentLocation` (`self.Mouth`)) (struct) 1.0 1.0 0.0 null null null null)))))))))))
        (:`then_1`
          (if (> (`KismetMathLibrary.VSize` (`CharacterMovementComponent.GetLastUpdateVelocity` (`self.CharacterMovement`))) 50.0)
            (`KismetSystemLibrary.Delay` (`KismetMathLibrary.RandomFloatInRange` 0.5 0.8))
            (`GameplayStatics.PlaySoundAtLocation` "/Game/Audio/Cues/C_GhoulEngage.C_GhoulEngage" _returnvalue_2 (struct) 1.0 1.0 0.0 null null null null)
            (else
              (`KismetSystemLibrary.Delay` (`KismetMathLibrary.RandomFloatInRange` 0.7 2.0))
              (`GameplayStatics.PlaySoundAtLocation` "/Game/Audio/Cues/C_GhoulAmbient.C_GhoulAmbient" _returnvalue_2 (struct) 1.0 1.0 0.0 null null null null))))))))

(event `self.BP_HealthComponent.OnDeath`
  (bind (_returnvalue_roll _returnvalue_pitch _returnvalue_yaw) (`KismetMathLibrary.BreakRotator` (`self.K2_GetActorRotation`)))
  (set `self.IsSpawning` true)
  (`PrimitiveComponent.SetCollisionEnabled` (`self.CapsuleComponent`) "NoCollision")
  (set `self.DeathYaw` _returnvalue_yaw)
  (set `self.IsDead` true)
  (`|ExecutionSequence`
    (:`then_0`
      (`KismetSystemLibrary.Delay` 10.0)
      (`self.K2_DestroyActor`))
    (:`then_1`
      (`/Engine/EditorBlueprintResources/StandardMacros.Gate` false :!label _label_3
        (:`Exit`
          (`GameplayStatics.PlaySoundAtLocation` "/Game/Audio/Cues/C_GhoulAmbient.C_GhoulAmbient" (`SceneComponent.K2_GetComponentLocation` (`self.Mouth`)) (struct) 1.0 1.0 0.0 null null null null)
          (goto _label_3 :!via `Close`))))))

(event `self.BP_HealthComponent.OnDamage`
  (params (Amount :type "Float (double-precision)") (Source :type "Actor Object Reference") (Direction :type "Vector Structure"))
  (`GameplayStatics.PlaySoundAtLocation` "/Game/Audio/Cues/C_GhoulHurt.C_GhoulHurt" (`SceneComponent.K2_GetComponentLocation` (`self.Mouth`)) (struct) 1.0 1.0 0.0 null null null null))

(fn `UserConstructionScript`
  (`parent.UserConstructionScript`))