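; BP_WitchHouse is an enemy spawner building that starts producing BP_SickleLantern enemies once the player enters its trigger.
; After activation, Tick feeds a random Delay of several seconds that acts as a repeating timer, with no shutoff in this graph.
; Each cycle swings the door open via a timeline, spawns an enemy at SpawnPoint with yaw opposite the house's, then closes the door.
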(event `self.Trigger.OnActorBeginOverlap`
  (params (OverlappedActor :type "Actor Object Reference") (OtherActor :type "Actor Object Reference"))
  (cast `/Game/Blueprints/BP_PlayerCharacter` OtherActor)
  (set `self.IsSpawning` true))

(event `self.ReceiveTick`
  (params (DeltaSeconds :type "Float (single-precision)"))
  (if (`self.IsSpawning`)
    (`KismetSystemLibrary.Delay` (`KismetMathLibrary.RandomFloatInRange` 7.0 12.0))
    (`self.SpawnSequence`)))

(event `OpenDoor`
  (bind (_direction _yaw) (`Timeline|OpenAnim` :!via `PlayFromStart` :!label _label)
    (:`Update`
      (`SceneComponent.K2_SetRelativeRotation` (`self.Door`) (`KismetMathLibrary.MakeRotator` 0.0 0.0 (`KismetMathLibrary.Lerp` 90.0 -10.0 _yaw)) false false))))

(event `CloseDoor`
  (goto _label :!via `ReverseFromEnd`))

(event `SpawnEnemy`
  (bind (_returnvalue_roll _returnvalue_pitch _returnvalue_yaw) (`KismetMathLibrary.BreakRotator` (`self.K2_GetActorRotation`)))
  (bind _returnvalue (`|SpawnActorFromClass` "/Game/Blueprints/BP_SickleLantern.BP_SickleLantern_C" (`KismetMathLibrary.MakeTransform` (0.0 0.0 0.0)) "AlwaysSpawn" "MultiplyWithRoot" null null))
  (`self.K2_SetActorLocationAndRotation` _returnvalue (`SceneComponent.K2_GetComponentLocation` (`self.SpawnPoint`)) (`KismetMathLibrary.MakeRotator` 0.0 0.0 (+ _returnvalue_yaw 180.0)) false true))

(event `SpawnSequence`
  (`self.OpenDoor`)
  (`KismetSystemLibrary.Delay` 0.2)
  (`self.SpawnEnemy`)
  (`KismetSystemLibrary.Delay` 3.0)
  (`self.CloseDoor`))

(fn `UserConstructionScript`)