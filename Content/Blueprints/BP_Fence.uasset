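; BP_Fence is a spline-driven fence actor that lays fence meshes along an editable path.
; Its construction script adds a spline mesh component for each segment between adjacent spline points, bending the SM_FenceStrip mesh along X to match each segment's local positions and tangents.
; Each generated segment has query and physics collision enabled, so the fence acts as a solid barrier.
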(fn `UserConstructionScript`
  (bind _spline (`self.Spline`))
  (for _index (range (+ (- (`SplineComponent.GetNumberOfSplinePoints` (`self.Spline`)) 2) 1))
    (bind _returnvalue (`AddComponent|NODE_AddSplineMeshComponent-0`))
    (`SplineMeshComponent.SetForwardAxis` _returnvalue "X" true)
    (bind _returnvalue_2 (+ _index 1))
    (`SplineMeshComponent.SetStartAndEnd` _returnvalue (`SplineComponent.GetLocationAtSplinePoint` _spline _index "Local") (`SplineComponent.GetTangentAtSplinePoint` _spline _index "Local") (`SplineComponent.GetLocationAtSplinePoint` _spline _returnvalue_2 "Local") (`SplineComponent.GetTangentAtSplinePoint` _spline _returnvalue_2 "Local") true)
    (`StaticMeshComponent.SetStaticMesh` _returnvalue "/Game/Meshes/SM_FenceStrip.SM_FenceStrip")
    (`PrimitiveComponent.SetCollisionEnabled` _returnvalue "QueryAndPhysics")))