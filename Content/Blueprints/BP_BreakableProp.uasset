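; BP_BreakableProp is a prop that breaks the first time it takes any damage.
; The construction script applies the configurable mesh to its static mesh component.
; On damage, a dead flag blocks repeat triggers, then it restarts the FX component with the break effect, plays a sound at its location and hides the mesh and its shadow.
; The actor destroys itself after a short delay.
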(event `self.ReceiveAnyDamage`
  (params (Damage :type "Float (single-precision)") (DamageType :type "DamageType Object Reference") (InstigatedBy :type "Controller Object Reference") (DamageCauser :type "Actor Object Reference"))
  (bind _fx (`self.FX`))
  (bind _staticmesh (`self.StaticMesh`))
  (if (not (`self.IsDead`))
    (set `self.IsDead` true)
    (`|ExecutionSequence`
      (:`then_0`
        (`NiagaraComponent.SetAsset` _fx (`self.BreakFX`) true)
        (`NiagaraComponent.ResetSystem` _fx))
      (:`then_1`
        (`GameplayStatics.PlaySoundAtLocation` (`self.BreakSound`) (`self.K2_GetActorLocation`) (struct) 1.0 1.0 0.0 null null null null))
      (:`then_2`
        (`SceneComponent.ToggleVisibility` _staticmesh false)
        (`PrimitiveComponent.SetCastShadow` _staticmesh false))
      (:`then_3`
        (`KismetSystemLibrary.Delay` 5.0)
        (`self.K2_DestroyActor`)))))

(fn `UserConstructionScript`
  (`StaticMeshComponent.SetStaticMesh` (`self.StaticMesh`) (`self.Mesh`)))