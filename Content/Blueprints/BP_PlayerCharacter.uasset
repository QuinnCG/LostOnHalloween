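; First-person player character with Enhanced Input movement, look, crouch and a melee attack.
; Tick plays footsteps at intervals while moving and sets walk speeds from HandGrabCount: grabs slow walking, while no grabs zero crouched speed.
; Cooldown-gated attack montage uses its "Damage" notify to capsule-trace from the camera, playing hit sounds and applying point damage.
; Crouch events offset camera height, and health component death only prints a message.
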(event `EnhancedInput|/Game/Blueprints/Input/IA_MoveForward`
  (params (ActionValue :type "Float (double-precision)") (ElapsedSeconds :type "Float (double-precision)") (TriggeredSeconds :type "Float (double-precision)") (InputAction :type "InputAction Object Reference" :default "/Game/Blueprints/Input/IA_MoveForward.IA_MoveForward"))
  (:`Triggered`
    (`self.AddMovementInput` (`self.GetActorForwardVector`) ActionValue))
  (:`Started`
    (if (== (`KismetMathLibrary.VSize` (`CharacterMovementComponent.GetLastUpdateVelocity` (`self.CharacterMovement`))) 0.0) :!label _label
      (`self.PlayFootstep`))))

(event `EnhancedInput|/Game/Blueprints/Input/IA_MoveRight`
  (params (ActionValue :type "Float (double-precision)") (ElapsedSeconds :type "Float (double-precision)") (TriggeredSeconds :type "Float (double-precision)") (InputAction :type "InputAction Object Reference" :default "/Game/Blueprints/Input/IA_MoveRight.IA_MoveRight"))
  (:`Triggered`
    (`self.AddMovementInput` (`self.GetActorRightVector`) ActionValue))
  (:`Started`
    (goto _label)))

(event `EnhancedInput|/Game/Blueprints/Input/IA_LookUp`
  (params (ActionValue :type "Float (double-precision)") (ElapsedSeconds :type "Float (double-precision)") (TriggeredSeconds :type "Float (double-precision)") (InputAction :type "InputAction Object Reference" :default "/Game/Blueprints/Input/IA_LookUp.IA_LookUp"))
  (:`Triggered`
    (`self.AddControllerPitchInput` (* ActionValue (`self.LookSensitivity`)))))

(event `EnhancedInput|/Game/Blueprints/Input/IA_LookRight`
  (params (ActionValue :type "Float (double-precision)") (ElapsedSeconds :type "Float (double-precision)") (TriggeredSeconds :type "Float (double-precision)") (InputAction :type "InputAction Object Reference" :default "/Game/Blueprints/Input/IA_LookRight.IA_LookRight"))
  (:`Triggered`
    (`self.AddControllerYawInput` (* ActionValue (`self.LookSensitivity`)))))

(event `EnhancedInput|/Game/Blueprints/Input/IA_Crouch`
  (params (ActionValue :type Boolean) (ElapsedSeconds :type "Float (double-precision)") (TriggeredSeconds :type "Float (double-precision)") (InputAction :type "InputAction Object Reference" :default "/Game/Blueprints/Input/IA_Crouch.IA_Crouch"))
  (:`Started`
    (`self.Crouch`))
  (:`Canceled`
    (`self.UnCrouch` :!label _label_2))
  (:`Completed`
    (goto _label_2)))

(event `self.K2_OnEndCrouch`
  (params (HalfHeightAdjust :type "Float (single-precision)") (ScaledHalfHeightAdjust :type "Float (single-precision)"))
  (bind (_relativelocation_x _relativelocation_y _relativelocation_z) (`KismetMathLibrary.BreakVector` (`SceneComponent.RelativeLocation` (`self.Camera`))))
  (`SceneComponent.K2_SetRelativeLocation` (`self.Camera`) (`KismetMathLibrary.MakeVector` _relativelocation_x _relativelocation_y (+ _relativelocation_z HalfHeightAdjust)) false false))

(event `self.K2_OnStartCrouch`
  (params (HalfHeightAdjust :type "Float (single-precision)") (ScaledHalfHeightAdjust :type "Float (single-precision)"))
  (bind (_relativelocation_x _relativelocation_y _relativelocation_z) (`KismetMathLibrary.BreakVector` (`SceneComponent.RelativeLocation` (`self.Camera`))))
  (`SceneComponent.K2_SetRelativeLocation` (`self.Camera`) (`KismetMathLibrary.MakeVector` _relativelocation_x _relativelocation_y (- _relativelocation_z HalfHeightAdjust)) false false))

(event `EnhancedInput|/Game/Blueprints/Input/IA_PrimaryAction`
  (params (ActionValue :type Boolean) (ElapsedSeconds :type "Float (double-precision)") (TriggeredSeconds :type "Float (double-precision)") (InputAction :type "InputAction Object Reference" :default "/Game/Blueprints/Input/IA_PrimaryAction.IA_PrimaryAction"))
  (bind _returnvalue (`self.GetController`))
  (bind _returnvalue_2 (`SceneComponent.K2_GetComponentLocation` (`self.Camera`)))
  (:`Started`
    (if (> (`KismetSystemLibrary.GetGameTimeInSeconds`) (`self.NextAttackTime`))
      (bind _notifyname (`|PlayMontage` (`self.Arms`) "/Game/Animations/M_PlayerAttack.M_PlayerAttack" 1.0 0.0 "Default")
        (:`then`
          (set `self.NextAttackTime` (+ (`KismetSystemLibrary.GetGameTimeInSeconds`) (`self.AttackInterval`))))
        (:`OnNotifyBegin`
          (bind _returnvalue_3 (== _notifyname "Damage"))
          (if _returnvalue_3
            (set `self.IsAttacking` true)
            (bind _outhits (`KismetSystemLibrary.CapsuleTraceMulti` _returnvalue_2 (+ _returnvalue_2 (* (`SceneComponent.GetForwardVector` (`self.Camera`)) (`self.AttackDistance`))) (`self.AttackRadius`) 35.0 "TraceTypeQuery1" true))
            (for _array_element _outhits
              (`|ExecutionSequence`
                (:`then_0`
                  (bind (_bblockinghit _binitialoverlap _time _distance _location _impactpoint _normal _impactnormal _physmat _hitactor) (`GameplayStatics.BreakHitResult` _array_element))
                  (`GameplayStatics.PlaySoundAtLocation` "/Game/Audio/Waves/S_Hit.S_Hit" _impactpoint (struct) (`KismetMathLibrary.RandomFloatInRange` 0.8 1.2) (`KismetMathLibrary.RandomFloatInRange` 0.8 1.2) 0.0 null null null null))
                (:`then_1`
                  (`GameplayStatics.ApplyPointDamage` _hitactor (`self.AttackDamage`) (`KismetMathLibrary.NegateVector` (`SceneComponent.GetForwardVector` (`self.Camera`))) _array_element _returnvalue _returnvalue))))))
        (:`OnNotifyEnd`
          (if _returnvalue_3
            (set `self.IsAttacking` false)))))))

(event `self.ReceiveBeginPlay`
  (`EnhancedInputSubsystemInterface.AddMappingContext` (pcsubsystem `EnhancedInputLocalPlayerSubsystem` (`GameplayStatics.GetPlayerController` 0)) "/Game/Blueprints/Input/IMC_Player.IMC_Player" 0 (struct)))

(event `self.ReceiveTick`
  (params (DeltaSeconds :type "Float (single-precision)"))
  (bind _charactermovement (`self.CharacterMovement`))
  (bind _returnvalue (> (`KismetMathLibrary.VSize` (`CharacterMovementComponent.GetLastUpdateVelocity` (`self.CharacterMovement`))) 0.0))
  (`|ExecutionSequence`
    (:`then_0`
      (if _returnvalue
        (`KismetSystemLibrary.Delay` (`self.FootstepInterval`))
        (if _returnvalue
          (`self.PlayFootstep`))))
    (:`then_1`
      (if (> (`self.HandGrabCount`) 0)
        (set `CharacterMovementComponent.MaxWalkSpeed` 150.0 _charactermovement)
        (set `CharacterMovementComponent.MaxWalkSpeedCrouched` 150.0 _charactermovement)
        (else
          (set `CharacterMovementComponent.MaxWalkSpeed` 450.0 _charactermovement)
          (set `CharacterMovementComponent.MaxWalkSpeedCrouched` 0.0 _charactermovement))))))

(event `self.BP_HealthComponent.OnDeath`
  (`KismetSystemLibrary.PrintText` "You died!"))

(event `PlayFootstep`
  (`GameplayStatics.PlaySoundAtLocation` "/Game/Audio/Metasounds/MS_Footstep.MS_Footstep" (`self.K2_GetActorLocation`) (struct) 0.5 0.6 0.0 null null null null))

(fn `UserConstructionScript`)