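; BP_HealthComponent is an actor component that tracks its owner's health and reports damage and death through event dispatchers.
; It resets Current to Max on BeginPlay and listens to the owner's OnTakeAnyDamage, applying damage through Remove, then broadcasting OnDamage with a zero direction.
; Add and Remove clamp health between zero and Max.
; Reaching zero unbinds all of the owner's OnTakeAnyDamage listeners and fires OnDeath, which precedes the final OnDamage.
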(event `self.ReceiveBeginPlay`
  (add `Actor.OnTakeAnyDamage` (`self.GetOwner`) (delegate `OnTakeAnyDamage_Event`))
  (set `self.Current` (`self.Max`)))

(event `OnTakeAnyDamage_Event`
  (params (DamagedActor :type "Actor Object Reference") (Damage :type "Float (single-precision)") (DamageType :type "DamageType Object Reference") (InstigatedBy :type "Controller Object Reference") (DamageCauser :type "Actor Object Reference"))
  (if (not (== (`self.Current`) 0.0))
    (`self.Remove` Damage)
    (`self.OnDamage` Damage InstigatedBy)
    (if (== (`self.Current`) 0.0)
      _)))

(fn `Add`
  (params (Amount :type "Float (double-precision)"))
  (set `self.Current` (`KismetMathLibrary.FMin` (+ Amount (`self.Current`)) (`self.Max`))))

(fn `Remove`
  (params (Amount :type "Float (double-precision)"))
  (bind _output_get (set `self.Current` (`KismetMathLibrary.FMax` (- (`self.Current`) Amount))))
  (if (== _output_get 0.0)
    (clear `Actor.OnTakeAnyDamage` (`self.GetOwner`))
    (`self.OnDeath`)))